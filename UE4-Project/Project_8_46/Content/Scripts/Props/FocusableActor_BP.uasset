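; FocusableActor_BP is a prop actor that can be focused and unfocused, tracking that state in a Focused flag.
; BeginFocus turns on custom depth rendering on its static mesh, sets the flag and returns the ActorType; EndFocus reverses both changes.
; GetType and IsFocused expose the type and state, the construction script starts it unfocused, and the event graph holds no logic.
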(event `self.ReceiveBeginPlay`)

(event `self.ReceiveActorBeginOverlap`
  (params (OtherActor :type "Actor Object Reference")))

(event `self.ReceiveTick`
  (params (DeltaSeconds :type "Float (single-precision)")))

(fn `BeginFocus`
  (returns (Type :type "/Game/Scripts/Props/EActorType_Enum Enum"))
  (`PrimitiveComponent.SetRenderCustomDepth` (`self.StaticMeshComponent`) true)
  (set `self.Focused` true)
  (return (`self.ActorType`)))

(fn `EndFocus`
  (`PrimitiveComponent.SetRenderCustomDepth` (`self.StaticMeshComponent`) false)
  (set `self.Focused` false))

(fn `GetType`
  (returns (ActorType :type "/Game/Scripts/Props/EActorType_Enum Enum"))
  (return (`self.ActorType`)))

(fn `IsFocused`
  (returns (IsFocused :type Boolean))
  (return (`self.Focused`)))

(fn `UserConstructionScript`
  (set `self.Focused` false) ; The component start is not focused
)